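; Doorway that shows a material effect and, when the player walks through, swaps it with the level's unbound post process material for a seamless transition.
; Each tick, a plane test on the follow camera's movement detects crossings from either side.
; MaterialsTable pairs door materials with post process materials in both lookup directions.
; The door mesh shifts away from nearby cameras to prevent clipping and sets translucent sort priority by player distance.
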(event `self.ReceiveBeginPlay`
  ;[0.5241 0.5806 1] Store the post process volume for future use
  (bind _outactors (`GameplayStatics.GetAllActorsOfClass` "/Script/Engine.PostProcessVolume"))
  (bind _output (`|GetArrayItem` _outactors))
  (`/Engine/EditorBlueprintResources/StandardMacros.IsValid` _output
    (:`Is Valid`
      (bind _output_get (set `self.PostProcessVolume` _output))
      (if (`PostProcessVolume.bUnbound` _output_get)
        ;[0.4351 0.5462 1] We need access to the player camera location to make this seamless. For reasons unknown to me, the camera location from the camera manager lags behind by a few frames which is enough to break the effect. So that is why I am doing a hard cast to a player character here.
        ;;[1 0.3451 0.3892] Replace cast here with the character you will be using
        (bind _asbp_example_character (cast `/Game/PP_Door_Effect/Demo/ThirdPerson/Blueprints/BP_ExampleCharacter` (`GameplayStatics.GetPlayerCharacter` 0))
          (:`then`
            (set `self.CharacterCamera` (`/Game/PP_Door_Effect/Demo/ThirdPerson/Blueprints/BP_ExampleCharacter.FollowCamera` _asbp_example_character)))
          (:`CastFailed`
            (`KismetSystemLibrary.PrintString` "CAST TO CHARACTER FAILED. BE SURE TO CAST TO THE CHARACTER YOU WILL BE USING ON BEGIN PLAY SEGMENT" true true (struct :`R` 1.0 :`B` 0.020919 :`A` 1.0) 10.0)
            (set `self.isValid` false)))
        (else
          (`KismetSystemLibrary.PrintString` "POST PROCESS VOLUME IS NOT UNBOUND. EFFECT WILL MOST LIKELY BREAK DOWN" true true (struct :`R` 1.0 :`B` 0.020919 :`A` 1.0) 10.0)
          (set `self.isValid` false))))
    (:`Is Not Valid`
      (`KismetSystemLibrary.PrintString` "NO POST PROCESS VOLUME DETECTED. EFFECT WILL NOT WORK" true true (struct :`R` 1.0 :`B` 0.020919 :`A` 1.0) 10.0)
      (set `self.isValid` false))))

(event `self.ReceiveTick`
  (params (DeltaSeconds :type "Float (single-precision)"))
  (bind (_value _returnvalue) (`BlueprintMapLibrary.Map_Find` (`self.MaterialsTable`) (`self.DoorMaterial`)))
  (if (`self.isValid`)
    (`self.AdjustPriority`)
    (if (`PrimitiveComponent.IsOverlappingActor` (`self.PlayerDetection`) (`GameplayStatics.GetPlayerCharacter` 0))
      (`self.PreventPlaneClipping`)
      (bind _iscrossing1 (`self.HasCrossedDoor`))
      (if _iscrossing1
        ;[0.5284 0.6322 1] Finds and stores the post process material for future use before we override the door material in the next function
        (if _returnvalue
          (set `self.NewPostProcessMAT` _value)
          (`self.SetDoorMaterial`)
          (`self.SetPostProcessMaterial`)
          (else
            (`KismetSystemLibrary.PrintString` "COULDN'T FIND THE MATERIAL IN THE MATERIAL TABLE MAP. BE SURE TO INCLUDE IN THE TABLE MAP" true true (struct :`R` 1.0 :`B` 0.020919 :`A` 1.0) 10.0))))
      (else
        (set `self.IsOverlapping` false)))))

(fn `AdjustPriority`
  ;[0.3102 0.5602 1] This ensures when multiple doors are in the level, that the further doorway material will always appear on top
  (`PrimitiveComponent.SetTranslucentSortPriority` (`self.Entry`) (`KismetMathLibrary.FTrunc` (`KismetMathLibrary.Vector_Distance` (`self.K2_GetActorLocation`) (`self.K2_GetActorLocation` (`GameplayStatics.GetPlayerCharacter` 0))))))

(fn `HasCrossedDoor`
  (returns (IsCrossing1 :type Boolean))
  (locals (IsInFront :type Boolean) (DoorPlane :type "Plane Structure") (IsIntersecting :type Boolean :default false) (IsCrossing :type Boolean :default false))
  (set `local.IsInFront` (>= (`KismetMathLibrary.Dot_VectorVector` (`SceneComponent.GetForwardVector` (`self.ForwardDirection`)) (- (`SceneComponent.K2_GetComponentLocation` (`self.CharacterCamera`)) (`self.K2_GetActorLocation`))) 0.0))
  (bind _output_get (set `local.DoorPlane` (`KismetMathLibrary.MakePlaneFromPointAndNormal` (`self.K2_GetActorLocation`) (`SceneComponent.GetForwardVector` (`self.ForwardDirection`)))))
  (set `local.IsIntersecting` (`.ReturnValue` (`KismetMathLibrary.LinePlaneIntersection` (`SceneComponent.K2_GetComponentLocation` (`self.CharacterCamera`)) (`self.LastPosition`) _output_get)))
  ;[0.2937 0.562 1] Determines if player crossed door from either side of door
  (set `local.IsCrossing` (or (and (`local.IsIntersecting`) (not (`local.IsInFront`)) (`self.LastInFront`) (`self.IsOverlapping`)) (and (`local.IsIntersecting`) (`local.IsInFront`) (not (`self.LastInFront`)) (`self.IsOverlapping`))))
  (set `self.LastInFront` (`local.IsInFront`))
  (set `self.LastPosition` (`SceneComponent.K2_GetComponentLocation` (`self.CharacterCamera`)))
  (set `self.IsOverlapping` true)
  (return (`local.IsCrossing`)))

(fn `PreventPlaneClipping`
  (bind _returnvalue (`KismetMathLibrary.Dot_VectorVector` (`SceneComponent.GetForwardVector` (`self.ForwardDirection`)) (- (`SceneComponent.K2_GetComponentLocation` (`self.CharacterCamera`)) (`self.K2_GetActorLocation`))))
  ;[0.3267 0.3819 1] This function exists to simply push the door mesh back ever so slightly from the player if they are right in front of it. This helps to prevent the camera from clipping through the mesh and ruin the effect
  (if (and (>= _returnvalue -3.0) (<= _returnvalue 0.0))
    ;;[1 1 1] Push mesh back if player is too close
    (`SceneComponent.K2_SetRelativeLocation` (`self.Entry`) (3.0 0.0 0.0) false false)
    (elif (and (>= _returnvalue 0.0) (<= _returnvalue 3.0))
      ;;[1 1 1] Push mesh back if player is too close
      (`SceneComponent.K2_SetRelativeLocation` (`self.Entry`) (-3.0 0.0 0.0) false false)
      (else
        (`SceneComponent.K2_SetRelativeLocation` (`self.Entry`) (0.0 0.0 0.0) false false)))))

(fn `SetDoorMaterial`
  (bind _array (break `WeightedBlendables` (`.WeightedBlendables` (break `PostProcessSettings` (`PostProcessVolume.Settings` (`self.PostProcessVolume`))))))
  (if (> (`KismetArrayLibrary.Array_Length` _array) 0)
    ;[0.639 0.7222 1] From the post process material, we will find the corresponding door material in our Materials Variable Table
    (bind _values (`BlueprintMapLibrary.Map_Values` (`self.MaterialsTable`)))
    (bind _keys (`BlueprintMapLibrary.Map_Keys` (`self.MaterialsTable`)))
    (bind _output (`|GetArrayItem` _keys (`KismetArrayLibrary.Array_Find` _values (cast `MaterialInterface` (`.Object` (break `WeightedBlendable` (`|GetArrayItem` _array))) :!pure true))))
    (`/Engine/EditorBlueprintResources/StandardMacros.IsValid` _output
      (:`Is Valid`
        (`PrimitiveComponent.SetMaterial` (`self.Entry`) 0 _output)
        (set `self.DoorMaterial` _output))
      (:`Is Not Valid`
        (`KismetSystemLibrary.PrintString` "COULDN'T FIND THE MATERIAL IN THE MATERIAL TABLE MAP. BE SURE TO INCLUDE IN THE TABLE MAP" true true (struct :`R` 1.0 :`B` 0.020919 :`A` 1.0) 10.0)))
    (else
      ;[0.5159 0.643 1] If no post process material is detected, which will happen when entering a door for the first time, then we will set it to the default material we created
      (set `self.DoorMaterial` "/Game/PP_Door_Effect/Materials/Door_Materials/Shader_Default.Shader_Default")
      (`PrimitiveComponent.SetMaterial` (`self.Entry`) 0 "/Game/PP_Door_Effect/Materials/Door_Materials/Shader_Default.Shader_Default"))))

(fn `SetPostProcessMaterial`
  ;[0.3881 0.4988 1] Set the material of the post process volume to the material we saved into the New Post Process MAT earlier
  (`KismetArrayLibrary.Array_Set` (`.Array` (break `WeightedBlendables` (`.WeightedBlendables` (break `PostProcessSettings` (`PostProcessVolume.Settings` (`self.PostProcessVolume`)))))) 0 (make `WeightedBlendable` 1.0 (`self.NewPostProcessMAT`)) true))

(fn `UserConstructionScript`
  (`PrimitiveComponent.SetMaterial` (`self.Entry`) 0 (`self.DoorMaterial`)))